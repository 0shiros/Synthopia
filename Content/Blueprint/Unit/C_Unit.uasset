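; Base Character for a team-owned, selectable combat unit, with health, damage, attack rate, move speed and type loaded from a UnitData struct.
; Action sends Attacked messages to a target, gated by a game-time cooldown.
; Attacked passes the aggressor to the unit's controller as its target, subtracts health and destroys the unit at zero.
; It also toggles a selection marker and finds its owning player's pawn by matching PC_Camera team index.
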(event `/Game/Blueprint/Unit/Interface/I_Unit.ToggleFocus`
  (params (isFocus :type Boolean))
  ; Show if Selected
  (`SceneComponent.SetVisibility` (`self.Focus`) isFocus false))

(event `/Game/Blueprint/Unit/Interface/I_Unit.Action`
  (params (Target :type "Object Object Reference"))
  ; To attack
  (if (`self.VerifyCooldown`)
    (`self.ResetCooldown`)
    (message `/Game/Blueprint/Interface/I_Selectable.Attacked` Target self (`self.Damage`))))

(event `/Game/Blueprint/Interface/I_Selectable.Attacked`
  (params (Agressor :type "Actor Object Reference") (Damage :type Integer))
  ; When is attacked
  (`/Engine/EditorBlueprintResources/StandardMacros.IsValid` (`self.Agressor`)
    (:`Is Valid`
      _)
    (:`Is Not Valid`
      (bind _output_get (set `self.Agressor` Agressor))))
  (message `/Game/Blueprint/Unit/AIController/Interface/I_UnitController.SetTarget` (`self.GetController`) _output_get)
  (bind _output_get_2 (set `self.Health` (- (`self.Health`) Damage)))
  (if (<= _output_get_2 0)
    (`self.K2_DestroyActor`)))

(event `/Game/Blueprint/Unit/Interface/I_Unit.SetIndexTeam`
  (params (IndexTeam :type Byte))
  ; Set IndexTeam Unit
  (set `self.TeamIndex` IndexTeam))

(fn `GetPlayer`
  (returns (ReturnValue :type "Pawn Object Reference"))
  (locals (PlayerToOutput :type "/Game/Blueprint/PlayerController/PC_Camera Object Reference"))
  (bind _outactors (`GameplayStatics.GetAllActorsOfClass` "/Game/Blueprint/PlayerController/PC_Camera.PC_Camera_C"))
  (for _array_element _outactors
    (if (== (`/Game/Blueprint/PlayerController/PC_Camera.TeamIndex` _array_element) (`self.TeamIndex`))
      (set `local.PlayerToOutput` _array_element)
      (break)))
  (return (`Controller.K2_GetPawn` (`local.PlayerToOutput`))))

(fn `GetTeamIndex`
  (returns (TeamIndex :type Byte))
  (return (`self.TeamIndex`)))

(fn `GetTimeToCreate`
  (returns (TimeToCreate :type Integer))
  (return (`self.TimeToCreate`)))

(fn `ResetCooldown`
  (set `self.LastTime` (`GameplayStatics.GetTimeSeconds`)))

(fn `SetUnit`
  (params (UnitData :type "/Game/Blueprint/UnitType/DataAsset/DA_UnitData Object Reference"))
  (set `self.Health` (`/Game/Blueprint/UnitType/DataAsset/DA_UnitData.Health` (`local.UnitData`)))
  (set `self.Damage` (`/Game/Blueprint/UnitType/DataAsset/DA_UnitData.Damage` (`local.UnitData`)))
  (set `self.TimeBetweenAttacks` (`/Game/Blueprint/UnitType/DataAsset/DA_UnitData.TimeBetweenAttacks` (`local.UnitData`)))
  (set `CharacterMovementComponent.MaxWalkSpeed` (* (`/Game/Blueprint/UnitType/DataAsset/DA_UnitData.MoveSpeed` (`local.UnitData`)) 100.0) (`self.CharacterMovement`))
  (set `self.Type` (`/Game/Blueprint/UnitType/DataAsset/DA_UnitData.Type` (`local.UnitData`))))

(fn `UserConstructionScript`)

(fn `VerifyCooldown`
  (returns (ReturnValue :type Boolean))
  (return (< (`self.TimeBetweenAttacks`) (- (`GameplayStatics.GetTimeSeconds`) (`self.LastTime`)))))