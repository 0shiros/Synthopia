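; Game HUD that draws a drag-selection box and gathers the units inside it as a new army.
; Separate events feed in the start and current mouse positions and the drawing state.
; While drawing, DrawHUD renders a translucent green rectangle once both axes pass a small drag threshold, querying it for C_Unit actors.
; A false CanDrawRect call passes the selection to the owning player controller via NewArmyMessage, then clears it.
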(event `self.ReceiveDrawHUD`
  (params (SizeX :type Integer) (SizeY :type Integer))
  (bind (_start_mouse_position_x _start_mouse_position_y) (`KismetMathLibrary.BreakVector2D` (`self.Start Mouse Position`)))
  (bind (_end_mouse_position_x _end_mouse_position_y) (`KismetMathLibrary.BreakVector2D` (`self.End Mouse Position`)))
  (bind (_returnvalue_x _returnvalue_y) (`KismetMathLibrary.BreakVector2D` (- (`self.Start Mouse Position`) (`self.End Mouse Position`))))
  (if (`self.Can Draw`)
    (if (and (or (> _returnvalue_x 25.0) (< _returnvalue_x -25.0)) (or (> _returnvalue_y 25.0) (< _returnvalue_y -25.0)))
      (`self.DrawRect` (struct :`R` 0.15 :`G` 1.0 :`B` 0.25 :`A` 0.5) _start_mouse_position_x _start_mouse_position_y (- _end_mouse_position_x _start_mouse_position_x) (- _end_mouse_position_y _start_mouse_position_y))
      (set `self.NewArmy` (`self.GetActorsInSelectionRectangle` "/Game/Blueprint/Unit/C_Unit.C_Unit_C" (`self.Start Mouse Position`) (`self.End Mouse Position`) false)))))

(event `/Game/Blueprint/HUD/Interface/I_HUD.CanDrawRect`
  (params (CanDraw :type Boolean))
  (bind _newarmy (`self.NewArmy`))
  (if CanDraw
    (set `self.Can Draw` true)
    (else
      (message `/Game/Blueprint/PlayerController/Interface/I_PlayerControllerCamera.NewArmy` (`self.GetOwningPlayerController`) _newarmy)
      (`KismetArrayLibrary.Array_Clear` _newarmy))))

(event `/Game/Blueprint/HUD/Interface/I_HUD.FirstMousePosition`
  (params (StartMousePosition :type "Vector2D Structure"))
  (set `self.Start Mouse Position` StartMousePosition))

(event `/Game/Blueprint/HUD/Interface/I_HUD.UpdateMousePosition`
  (params (EndMousePosition :type "Vector2D Structure"))
  (set `self.End Mouse Position` EndMousePosition))

(fn `UserConstructionScript`)