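; RTS player controller that drives the P_Camera pawn (keys, edge scrolling, ortho zoom) and handles units and buildings.
; Click or HUD drag-box selection fills an Army of team-owned AI controllers, expanded through A_UnitGroup, for grid-offset move or attack orders.
; Building preview follows the cursor on a looping timer with rotation, optional grid snap and Shift repeat placement.
; Select, Order and Building input mapping contexts are swapped by state, while another timer drives hover highlighting.
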(event `Start`
  ; Setup PlayerController
  (`EnhancedInputSubsystemInterface.AddMappingContext` (pcsubsystem `EnhancedInputLocalPlayerSubsystem` self) "/Game/Blueprint/PlayerController/Input/IMC/Camera/IMC_Camera.IMC_Camera" 0 (struct))
  (bind _asp_camera (cast `/Game/Blueprint/Camera/P_Camera` (`self.K2_GetPawn`)))
  (bind _output_get (set `self.As P Camera` _asp_camera))
  (set `self.CameraZoom` (`CameraComponent.OrthoWidth` (`/Game/Blueprint/Camera/P_Camera.Camera` _output_get)))
  (`WidgetBlueprintLibrary.SetInputMode_GameAndUIEx` self null "LockAlways" false)
  (set `self.bShowMouseCursor` true)
  (bind _returnvalue (`KismetSystemLibrary.K2_SetTimer` null "HoverUnit" 0.03 true))
  (set `self.HowerUnitTimer` _returnvalue)
  (`EnhancedInputSubsystemInterface.AddMappingContext` (subsystem `EnhancedInputLocalPlayerSubsystem`) "/Game/Blueprint/PlayerController/Input/IMC/Select/IMC_Select.IMC_Select" 0 (struct)))

(event `EnhancedInput|/Game/Blueprint/PlayerController/Input/Action/Camera/IAC_MoveCameraKeyboard`
  (params (ActionValue :type "Vector2D Structure") (ElapsedSeconds :type "Float (double-precision)") (TriggeredSeconds :type "Float (double-precision)") (InputAction :type "InputAction Object Reference" :default "/Game/Blueprint/PlayerController/Input/Action/Camera/IAC_MoveCameraKeyboard.IAC_MoveCameraKeyboard"))
  (bind _as_p_camera (`self.As P Camera`))
  ; Move Camera (ZQSD)
  (:`Triggered`
    (set `FloatingPawnMovement.MaxSpeed` (`/Game/Blueprint/Camera/P_Camera.DefaultMoveSpeed` _as_p_camera) (`/Game/Blueprint/Camera/P_Camera.FloatingPawnMovement` _as_p_camera))
    (`self.MoveForward` ActionValue_X)
    (`self.MoveRight` ActionValue_Y)))

(event `EnhancedInput|/Game/Blueprint/PlayerController/Input/Action/Camera/IAC_Zoom`
  (params (ActionValue :type "Float (double-precision)") (ElapsedSeconds :type "Float (double-precision)") (TriggeredSeconds :type "Float (double-precision)") (InputAction :type "InputAction Object Reference" :default "/Game/Blueprint/PlayerController/Input/Action/Camera/IAC_Zoom.IAC_Zoom"))
  ; Zoom (Mouse Wheel)
  (:`Triggered`
    (bind _result (`/Engine/EditorBlueprintResources/StandardMacros.NegateFloat` ActionValue)
      (:`  `
        (bind _output_get (set `self.CameraZoom` (`KismetMathLibrary.FClamp` (+ (* _result 100.0) (`self.CameraZoom`)) 1000.0 2500.0)))
        (`CameraComponent.SetOrthoWidth` (`/Game/Blueprint/Camera/P_Camera.Camera` (`self.As P Camera`)) _output_get)))))

(event `InputAxisKey|MouseY`
  (params (AxisValue :type "Float (single-precision)"))
  (bind (_returnvalue_x _returnvalue_y) (`KismetMathLibrary.BreakVector2D` (`WidgetLayoutLibrary.GetViewportSize`)))
  (bind _as_p_camera (`self.As P Camera`))
  (bind _returnvalue (/ (`self.GetMousePosition` self) _returnvalue_x))
  ; Move Camera to Limit Border (MousePosition)
  (if (> _returnvalue 0.98)
    (`self.MoveRight` 1.0)
    (set `FloatingPawnMovement.MaxSpeed` (`/Game/Blueprint/Camera/P_Camera.MaxMoveSpeed` _as_p_camera) (`/Game/Blueprint/Camera/P_Camera.FloatingPawnMovement` _as_p_camera) :!label _label)
    (elif (< _returnvalue 0.02)
      (`self.MoveRight` -1.0)
      (goto _label))))

(event `InputAxisKey|MouseX`
  (params (AxisValue :type "Float (single-precision)"))
  (bind (_returnvalue_x _returnvalue_y) (`KismetMathLibrary.BreakVector2D` (`WidgetLayoutLibrary.GetViewportSize`)))
  (bind _returnvalue (/ (`.LocationY` (`self.GetMousePosition` self)) _returnvalue_y))
  ; Move Camera to Limit Border (MousePosition)
  (if (> _returnvalue 0.98)
    (`self.MoveForward` -1.0)
    (goto _label)
    (elif (< _returnvalue 0.02)
      (`self.MoveForward` 1.0)
      (goto _label))))

(event `EnhancedInput|/Game/Blueprint/PlayerController/Input/Action/Select/IAC_Click`
  (params (ActionValue :type Boolean) (ElapsedSeconds :type "Float (double-precision)") (TriggeredSeconds :type "Float (double-precision)") (InputAction :type "InputAction Object Reference" :default "/Game/Blueprint/PlayerController/Input/Action/Select/IAC_Click.IAC_Click"))
  (bind _returnvalue (`self.GetHUD`))
  (bind _returnvalue_2 (`self.GetHUD`))
  (bind (_locationx _locationy) (`self.GetMousePosition`))
  (bind _returnvalue_3 (subsystem `EnhancedInputLocalPlayerSubsystem`))
  (bind _army (`self.Army`))
  (bind (_hitresult _returnvalue_4) (`self.GetHitResultUnderCursorForObjects` (`|MakeArray` "ObjectTypeQuery8" :!type "EObjectTypeQuery Enum")))
  (bind (_hitresult_2 _returnvalue_5) (`self.GetHitResultUnderCursorForObjects` (`|MakeArray` (cast `EObjectTypeQuery` 6))))
  (bind (_bblockinghit _binitialoverlap _time _distance _location _impactpoint _normal _impactnormal _physmat _hitactor) (`GameplayStatics.BreakHitResult` _hitresult))
  (bind (_bblockinghit_2 _binitialoverlap_2 _time_2 _distance_2 _location_2 _impactpoint_2 _normal_2 _impactnormal_2 _physmat_2 _hitactor_2) (`GameplayStatics.BreakHitResult` _hitresult_2))
  (bind _returnvalue_6 (`AIBlueprintHelperLibrary.GetAIController` _hitactor_2))
  ; Select Units (LeftClick)
  (:`Triggered`
    (message `/Game/Blueprint/HUD/Interface/I_HUD.UpdateMousePosition` _returnvalue_2 (`KismetMathLibrary.MakeVector2D` _locationx _locationy)))
  (:`Started`
    (message `/Game/Blueprint/HUD/Interface/I_HUD.FirstMousePosition` _returnvalue_2 (`KismetMathLibrary.MakeVector2D` _locationx _locationy))
    (message `/Game/Blueprint/HUD/Interface/I_HUD.CanDrawRect` _returnvalue_2 true))
  (:`Completed`
    (message `/Game/Blueprint/HUD/Interface/I_HUD.UpdateMousePosition` _returnvalue (0.0 0.0))
    (message `/Game/Blueprint/HUD/Interface/I_HUD.FirstMousePosition` _returnvalue (0.0 0.0))
    (message `/Game/Blueprint/HUD/Interface/I_HUD.CanDrawRect` _returnvalue false)
    (if (`self.HasArmy`)
      (set `self.HasArmy` false)
      (elif _returnvalue_5
        (bind _teamindex (message `/Game/Blueprint/Interface/I_Selectable.GetTeamIndex` _hitactor_2))
        (if (== _teamindex (`self.TeamIndex`))
          (bind _unitgroup (message `/Game/Blueprint/Unit/AIController/Interface/I_UnitController.GetUnitGroup` _returnvalue_6))
          (`/Engine/EditorBlueprintResources/StandardMacros.IsValid` _unitgroup
            (:`Is Valid`
              (bind _group (message `/Game/Blueprint/UnitGroup/Interface/I_UnitGroup.GetGroup` _unitgroup))
              (for _array_element _group
                (bind _selectedunit (message `/Game/Blueprint/Unit/AIController/Interface/I_UnitController.Selected` _array_element))
                (`KismetArrayLibrary.Array_AddUnique` (`self.Army`) _selectedunit)))
            (:`Is Not Valid`
              (bind _selectedunit_2 (message `/Game/Blueprint/Unit/AIController/Interface/I_UnitController.Selected` _returnvalue_6))
              (`KismetArrayLibrary.Array_AddUnique` (`self.Army`) _selectedunit_2)))
          (`EnhancedInputSubsystemInterface.AddMappingContext` _returnvalue_3 "/Game/Blueprint/PlayerController/Input/IMC/Order/IMC_Order.IMC_Order" 0 (struct)))
        (else
          (for _array_element_2 _army
            (message `/Game/Blueprint/Unit/AIController/Interface/I_UnitController.Deselected` _array_element_2))
          (`KismetArrayLibrary.Array_Clear` _army)
          (`EnhancedInputSubsystemInterface.RemoveMappingContext` _returnvalue_3 "/Game/Blueprint/PlayerController/Input/IMC/Order/IMC_Order.IMC_Order" (struct))
          (if _returnvalue_4
            (bind _teamindex_2 (message `/Game/Blueprint/Interface/I_Selectable.GetTeamIndex` _hitactor))
            (if (== _teamindex_2 (`self.TeamIndex`))
              (`/Game/Blueprint/HUD/HUD_Game.ShowUIBuilding` (cast `/Game/Blueprint/HUD/HUD_Game` (`self.GetHUD`) :!pure true) (cast `/Game/Blueprint/Building/A_Building` _hitactor :!pure true) true))
            (else
              (bind _ashud_game (cast `/Game/Blueprint/HUD/HUD_Game` (`self.GetHUD`)))
              (`/Game/Blueprint/HUD/HUD_Game.ShowUIBuilding` _ashud_game null false))))))))

(event `EnhancedInput|/Game/Blueprint/PlayerController/Input/Action/Order/IA_GiveOrder`
  (params (ActionValue :type Boolean) (ElapsedSeconds :type "Float (double-precision)") (TriggeredSeconds :type "Float (double-precision)") (InputAction :type "InputAction Object Reference" :default "/Game/Blueprint/PlayerController/Input/Action/Order/IA_GiveOrder.IA_GiveOrder"))
  (bind (_bblockinghit _binitialoverlap _time _distance _location _impactpoint _normal _impactnormal _physmat _hitactor) (`GameplayStatics.BreakHitResult` (`self.GetHitResultUnderCursorForObjects` (`|MakeArray` "ObjectTypeQuery6" :!type "EObjectTypeQuery Enum"))))
  (bind (_bblockinghit_2 _binitialoverlap_2 _time_2 _distance_2 _location_2 _impactpoint_2 _normal_2 _impactnormal_2 _physmat_2 _hitactor_2) (`GameplayStatics.BreakHitResult` (`self.GetHitResultUnderCursorForObjects` (`|MakeArray` "ObjectTypeQuery7" "ObjectTypeQuery8" :!type "EObjectTypeQuery Enum"))))
  ; Unit Move (RightClick)
  (:`Triggered`
    ;; Move To Click (maintain)
    (for (_array_element _array_index) (`self.Army`)
      (message `/Game/Blueprint/Unit/AIController/Interface/I_UnitController.CancelAction` _array_element false)
      (bind _returnvalue (+ (`KismetMathLibrary.MakeVector` (`KismetMathLibrary.Conv_IntToDouble` (* (/ _array_index 2) 150)) (`KismetMathLibrary.Conv_IntToDouble` (* (mod _array_index 2) 150))) (`.Location` (`GameplayStatics.BreakHitResult` (`self.GetHitResultUnderCursorByChannel` "TraceTypeQuery1")))))
      (`AIController.K2_SetFocalPoint` _array_element _returnvalue)
      (`|AIMoveTo` (`self.K2_GetPawn` _array_element) _returnvalue null)))
  (:`Completed`
    (`/Engine/EditorBlueprintResources/StandardMacros.IsValid` _hitactor
      (:`Is Valid`
        (for _array_element_2 (`self.Army`)
          (message `/Game/Blueprint/Unit/AIController/Interface/I_UnitController.CancelAction` _array_element_2 false)
          (message `/Game/Blueprint/Unit/AIController/Interface/I_UnitController.SetTarget` _array_element_2 _hitactor)))
      (:`Is Not Valid`
        ;; Move to click (One click)
        (bind _teamindex (message `/Game/Blueprint/Interface/I_Selectable.GetTeamIndex` _hitactor_2))
        (if (!= _teamindex (`self.TeamIndex`))
          (for _array_element_3 (`self.Army`)
            (message `/Game/Blueprint/Unit/AIController/Interface/I_UnitController.CancelAction` _array_element_3 false)
            (message `/Game/Blueprint/Unit/AIController/Interface/I_UnitController.SetTarget` _array_element_3 _hitactor_2))
          (else
            (for (_array_element_4 _array_index_2) (`self.Army`)
              (message `/Game/Blueprint/Unit/AIController/Interface/I_UnitController.CancelAction` _array_element_4 true)
              (message `/Game/Blueprint/Unit/AIController/Interface/I_UnitController.SetTarget` _array_element_4 null)
              (message `/Game/Blueprint/Unit/AIController/Interface/I_UnitController.MoveTo` _array_element_4 (+ (`KismetMathLibrary.MakeVector` (`KismetMathLibrary.Conv_IntToDouble` (* (/ _array_index_2 2) 150)) (`KismetMathLibrary.Conv_IntToDouble` (* (mod _array_index_2 2) 150))) (`.Location` (`GameplayStatics.BreakHitResult` (`self.GetHitResultUnderCursorByChannel` "TraceTypeQuery1"))))))))))))

(event `/Game/Blueprint/PlayerController/Interface/I_PlayerControllerCamera.NewArmy`
  (params (NewArmy :type "Array of Actor Object Reference (by ref)"))
  (bind _army (`self.Army`))
  ; Add Unit to Army
  (if (`KismetArrayLibrary.Array_IsEmpty` NewArmy)
    (if (not (`self.MoreOption`))
      (for _array_element _army
        (message `/Game/Blueprint/Unit/AIController/Interface/I_UnitController.Deselected` _array_element))
      (`KismetArrayLibrary.Array_Clear` _army)
      (`EnhancedInputSubsystemInterface.RemoveMappingContext` (subsystem `EnhancedInputLocalPlayerSubsystem`) "/Game/Blueprint/PlayerController/Input/IMC/Order/IMC_Order.IMC_Order" (struct))
      (set `self.HasArmy` false))
    (else
      (`KismetArrayLibrary.Array_Clear` (`self.Army`))
      (for _array_element_2 NewArmy
        (bind _selectedunit (message `/Game/Blueprint/Unit/AIController/Interface/I_UnitController.Selected` (`AIBlueprintHelperLibrary.GetAIController` _array_element_2)))
        (`KismetArrayLibrary.Array_AddUnique` (`self.Army`) _selectedunit))
      (`EnhancedInputSubsystemInterface.AddMappingContext` (subsystem `EnhancedInputLocalPlayerSubsystem`) "/Game/Blueprint/PlayerController/Input/IMC/Order/IMC_Order.IMC_Order" 0 (struct))
      (set `self.HasArmy` true)
      (for _array_element_3 (`self.Army`)
        (bind _unitgroup (message `/Game/Blueprint/Unit/AIController/Interface/I_UnitController.GetUnitGroup` _array_element_3))
        (`/Engine/EditorBlueprintResources/StandardMacros.IsValid` _unitgroup
          (:`Is Valid`
            (if (`KismetArrayLibrary.Array_IsEmpty` (`self.SelectedUnitGroup`))
              (`KismetArrayLibrary.Array_Add` (`self.SelectedUnitGroup`) _unitgroup)
              (bind _group (message `/Game/Blueprint/UnitGroup/Interface/I_UnitGroup.GetGroup` _unitgroup))
              (for _array_element_4 _group
                (bind _selectedunit_2 (message `/Game/Blueprint/Unit/AIController/Interface/I_UnitController.Selected` _array_element_4))
                (`KismetArrayLibrary.Array_AddUnique` (`self.Army`) _selectedunit_2))
              (else
                (for _array_element_5 (`self.SelectedUnitGroup`)
                  (set `self.IsNewGroup` (!= _unitgroup _array_element_5)))
                (if (`self.IsNewGroup`)
                  (`KismetArrayLibrary.Array_Add` (`self.SelectedUnitGroup`) _unitgroup)
                  (bind _group_2 (message `/Game/Blueprint/UnitGroup/Interface/I_UnitGroup.GetGroup` _unitgroup))
                  (for _array_element_6 _group_2
                    (bind _selectedunit_3 (message `/Game/Blueprint/Unit/AIController/Interface/I_UnitController.Selected` _array_element_6))
                    (`KismetArrayLibrary.Array_AddUnique` (`self.Army`) _selectedunit_3))))))))
      (`KismetArrayLibrary.Array_Clear` (`self.SelectedUnitGroup`)))))

(event `EnhancedInput|/Game/Blueprint/PlayerController/Input/Action/Camera/IAC_MoreOption`
  (params (ActionValue :type Boolean) (ElapsedSeconds :type "Float (double-precision)") (TriggeredSeconds :type "Float (double-precision)") (InputAction :type "InputAction Object Reference" :default "/Game/Blueprint/PlayerController/Input/Action/Camera/IAC_MoreOption.IAC_MoreOption"))
  ; MoreOptions (Shift)
  (:`Started`
    (set `self.MoreOption` true))
  (:`Completed`
    (set `self.MoreOption` false)))

(event `EnhancedInput|/Game/Blueprint/PlayerController/Input/Action/Building/IAC_BuildingConstruct`
  (params (ActionValue :type Boolean) (ElapsedSeconds :type "Float (double-precision)") (TriggeredSeconds :type "Float (double-precision)") (InputAction :type "InputAction Object Reference" :default "/Game/Blueprint/PlayerController/Input/Action/Building/IAC_BuildingConstruct.IAC_BuildingConstruct"))
  (bind _returnvalue (subsystem `EnhancedInputLocalPlayerSubsystem`))
  ; Place building (LeftClick)
  (:`Completed`
    (bind _canbuild (message `/Game/Blueprint/Building/Interface/I_Building.Build` (`self.BuildingPreview`)))
    (if _canbuild
      (if (`self.MoreOption`)
        (`self.CreateBuildingPreview` (`GameplayStatics.GetObjectClass` (`self.BuildingPreview`)))
        (else
          (`KismetSystemLibrary.K2_ClearAndInvalidateTimerHandle` (`self.BuildingPositionTimer`))
          (set `self.BuildingPreview` null)
          (`EnhancedInputSubsystemInterface.AddMappingContext` _returnvalue "/Game/Blueprint/PlayerController/Input/IMC/Select/IMC_Select.IMC_Select" 0 (struct))
          (`EnhancedInputSubsystemInterface.RemoveMappingContext` _returnvalue "/Game/Blueprint/PlayerController/Input/IMC/Building/IMC_Building.IMC_Building" (struct))
          (`KismetSystemLibrary.K2_UnPauseTimerHandle` (`self.HowerUnitTimer`)))))))

(event `EnhancedInput|/Game/Blueprint/PlayerController/Input/Action/Building/IAC_RotateBuilding`
  (params (ActionValue :type "Float (double-precision)") (ElapsedSeconds :type "Float (double-precision)") (TriggeredSeconds :type "Float (double-precision)") (InputAction :type "InputAction Object Reference" :default "/Game/Blueprint/PlayerController/Input/Action/Building/IAC_RotateBuilding.IAC_RotateBuilding"))
  (bind _buildingpreview (`self.BuildingPreview`))
  ; Rotation (A and E)
  (:`Started`
    (if (> ActionValue 0.0)
      (`self.K2_AddActorWorldRotation` _buildingpreview (struct :`Yaw` 30.0) false false)
      (else
        (`self.K2_AddActorWorldRotation` _buildingpreview (struct :`Yaw` -30.0) false false)))))

(event `EnhancedInput|/Game/Blueprint/PlayerController/Input/Action/Building/IAC_PrecisionConstruct`
  (params (ActionValue :type Boolean) (ElapsedSeconds :type "Float (double-precision)") (TriggeredSeconds :type "Float (double-precision)") (InputAction :type "InputAction Object Reference" :default "/Game/Blueprint/PlayerController/Input/Action/Building/IAC_PrecisionConstruct.IAC_PrecisionConstruct"))
  ; Set Building precisely
  (:`Started`
    (if (`self.PrecisionBuilding`)
      (set `self.PrecisionBuilding` false)
      (else
        (set `self.PrecisionBuilding` true)))))

(event `EnhancedInput|/Game/Blueprint/PlayerController/Input/Action/Order/IAC_MakeGroup`
  (params (ActionValue :type Boolean) (ElapsedSeconds :type "Float (double-precision)") (TriggeredSeconds :type "Float (double-precision)") (InputAction :type "InputAction Object Reference" :default "/Game/Blueprint/PlayerController/Input/Action/Order/IAC_MakeGroup.IAC_MakeGroup"))
  ; Group Units
  (:`Started`
    (if (`self.MoreOption`)
      ;; Destroy Group (Shift+G when selected)
      (for _array_element (`self.Army`)
        (bind _unitgroup (message `/Game/Blueprint/Unit/AIController/Interface/I_UnitController.GetUnitGroup` _array_element))
        (`/Engine/EditorBlueprintResources/StandardMacros.IsValid` _unitgroup
          (:`Is Valid`
            (`self.K2_DestroyActor` _unitgroup))))
      (else
        ;; Create Groups (G when selected)
        (bind _returnvalue (`|SpawnActorFromClass` "/Game/Blueprint/UnitGroup/A_UnitGroup.A_UnitGroup_C" (`KismetMathLibrary.MakeTransform` (0.0 0.0 0.0)) "Undefined" "MultiplyWithRoot" null (`self.Army`) null))
        (for _array_element_2 (`self.Army`)
          (bind _unitgroup_2 (message `/Game/Blueprint/Unit/AIController/Interface/I_UnitController.GetUnitGroup` _array_element_2))
          (`/Engine/EditorBlueprintResources/StandardMacros.IsValid` _unitgroup_2
            (:`Is Valid`
              (`self.K2_DestroyActor` _unitgroup_2))
            (:`Is Not Valid`
              _))
          (message `/Game/Blueprint/Unit/AIController/Interface/I_UnitController.SetUnitGroup` _array_element_2 _returnvalue))))))

(fn `BuildingPosition`
  (bind _buildingpreview (`self.BuildingPreview`))
  (bind (_bblockinghit _binitialoverlap _time _distance _location _impactpoint) (`GameplayStatics.BreakHitResult` (`self.GetHitResultUnderCursorForObjects` (`|MakeArray` "ObjectTypeQuery1" :!type "EObjectTypeQuery Enum"))))
  (bind (_returnvalue_x _returnvalue_y) (`KismetMathLibrary.BreakVector` (/ _impactpoint 100.0)))
  (if (== _impactpoint (0.0 0.0 0.0))
    (`self.SetActorHiddenInGame` _buildingpreview true)
    (else
      (`self.SetActorHiddenInGame` _buildingpreview false)
      (if (`self.PrecisionBuilding`)
        (`self.K2_SetActorLocation` _buildingpreview (`KismetMathLibrary.MakeVector` (* (`KismetMathLibrary.Round` _returnvalue_x) 100) (* (`KismetMathLibrary.Round` _returnvalue_y) 100)) false false)
        (else
          (`self.K2_SetActorLocation` _buildingpreview _impactpoint false false))))))

(fn `CreateBuildingPreview`
  (params (BuildingClass :type "/Game/Blueprint/Building/A_Building Class Reference") (IsNotMultipleConstruct :type Boolean))
  (bind _returnvalue (subsystem `EnhancedInputLocalPlayerSubsystem`))
  (bind _army (`self.Army`))
  (bind _howerunittimer (`self.HowerUnitTimer`))
  (for _array_element _army
    (message `/Game/Blueprint/Unit/AIController/Interface/I_UnitController.Deselected` _array_element))
  (`KismetArrayLibrary.Array_Clear` _army)
  (`EnhancedInputSubsystemInterface.RemoveMappingContext` (subsystem `EnhancedInputLocalPlayerSubsystem`) "/Game/Blueprint/PlayerController/Input/IMC/Order/IMC_Order.IMC_Order" (struct))
  (message `/Game/Blueprint/Unit/Interface/I_Unit.ToggleFocus` (`self.Focused`) false)
  (if (`local.IsNotMultipleConstruct`)
    (`/Engine/EditorBlueprintResources/StandardMacros.IsValid` (`self.BuildingPreview`)
      (:`Is Valid`
        (`KismetSystemLibrary.K2_UnPauseTimerHandle` _howerunittimer)
        (`EnhancedInputSubsystemInterface.AddMappingContext` _returnvalue "/Game/Blueprint/PlayerController/Input/IMC/Select/IMC_Select.IMC_Select" 0 (struct))
        (`EnhancedInputSubsystemInterface.RemoveMappingContext` _returnvalue "/Game/Blueprint/PlayerController/Input/IMC/Building/IMC_Building.IMC_Building" (struct))
        (`self.K2_DestroyActor` (`self.BuildingPreview`))
        (`KismetSystemLibrary.K2_ClearAndInvalidateTimerHandle` (`self.BuildingPositionTimer`))
        (set `self.BuildingPreview` null))
      (:`Is Not Valid`
        (`KismetSystemLibrary.K2_PauseTimerHandle` _howerunittimer :!label _label)
        (`EnhancedInputSubsystemInterface.AddMappingContext` _returnvalue "/Game/Blueprint/PlayerController/Input/IMC/Building/IMC_Building.IMC_Building" 0 (struct))
        (`EnhancedInputSubsystemInterface.RemoveMappingContext` _returnvalue "/Game/Blueprint/PlayerController/Input/IMC/Select/IMC_Select.IMC_Select" (struct))
        (bind _returnvalue_2 (`|SpawnActorFromClass` (`local.BuildingClass`) (`KismetMathLibrary.MakeTransform` (0.0 0.0 0.0)) "Undefined" "MultiplyWithRoot" null null))
        (set `self.BuildingPreview` _returnvalue_2)
        (bind _returnvalue_3 (`KismetSystemLibrary.K2_SetTimer` null "BuildingPosition" 0.03 true))
        (set `self.BuildingPositionTimer` _returnvalue_3)))
    (else
      (goto _label))))

(fn `GetArmy`
  (returns (Army :type "Array of AIController Object Reference"))
  (return (`self.Army`)))

(fn `GetMoreOptions`
  (returns (MoreOption :type Boolean))
  (return (`self.MoreOption`)))

(fn `GetTeamIndex`
  (returns (IndexTeam :type Byte))
  (return 0))

(fn `HoverUnit`
  (bind _returnvalue (`AIBlueprintHelperLibrary.GetAIController` (`self.Focused`)))
  (bind (_bblockinghit _binitialoverlap _time _distance _location _impactpoint _normal _impactnormal _physmat _hitactor) (`GameplayStatics.BreakHitResult` (`self.GetHitResultUnderCursorForObjects` (`|MakeArray` (cast `EObjectTypeQuery` 6)))))
  (bind _teamindex (message `/Game/Blueprint/Interface/I_Selectable.GetTeamIndex` _hitactor))
  (if (== _teamindex (`self.TeamIndex`))
    (if (== _hitactor (`self.Focused`))
      (bind _unitgroup (message `/Game/Blueprint/Unit/AIController/Interface/I_UnitController.GetUnitGroup` (`AIBlueprintHelperLibrary.GetAIController` (`self.Focused`))))
      (`/Engine/EditorBlueprintResources/StandardMacros.IsValid` _unitgroup
        (:`Is Valid`
          (message `/Game/Blueprint/UnitGroup/Interface/I_UnitGroup.FocusAll` _unitgroup true))
        (:`Is Not Valid`
          (message `/Game/Blueprint/Unit/Interface/I_Unit.ToggleFocus` (`self.Focused`) true)))
      (else
        (bind _isselected (message `/Game/Blueprint/Unit/AIController/Interface/I_UnitController.IsSelected` _returnvalue))
        (if (not _isselected)
          (bind _unitgroup_2 (message `/Game/Blueprint/Unit/AIController/Interface/I_UnitController.GetUnitGroup` _returnvalue))
          (`/Engine/EditorBlueprintResources/StandardMacros.IsValid` _unitgroup_2
            (:`Is Valid`
              (message `/Game/Blueprint/UnitGroup/Interface/I_UnitGroup.FocusAll` _unitgroup_2 false))
            (:`Is Not Valid`
              (message `/Game/Blueprint/Unit/Interface/I_Unit.ToggleFocus` (`self.Focused`) false))))
        (set `self.Focused` _hitactor)))))

(fn `MoveForward`
  (params (x :type "Float (double-precision)"))
  (bind (_returnvalue_roll _returnvalue_pitch _returnvalue_yaw) (`KismetMathLibrary.BreakRotator` (`self.GetControlRotation`)))
  (`Pawn.AddMovementInput` (`self.As P Camera`) (`KismetMathLibrary.GetForwardVector` (`KismetMathLibrary.MakeRotator` _returnvalue_roll 0.0 _returnvalue_yaw)) x false))

(fn `MoveRight`
  (params (y :type "Float (double-precision)"))
  (bind (_returnvalue_roll _returnvalue_pitch _returnvalue_yaw) (`KismetMathLibrary.BreakRotator` (`self.GetControlRotation`)))
  (`Pawn.AddMovementInput` (`self.As P Camera`) (`KismetMathLibrary.GetRightVector` (`KismetMathLibrary.MakeRotator` 0.0 0.0 _returnvalue_yaw)) y false))

(fn `UserConstructionScript`)